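; BP_Cube is an actor that moves along its own up axis around its starting position, driven by a float curve.
; BeginPlay stores the start location as Origin.
; Each Tick samples the NewVar curve at the current game time, scales it and sets the location to Origin plus that up-vector offset, without sweep.
; The overlap event and construction script are empty.
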(event EventBeginPlay
  (Variables|Default|SetOrigin (Transformation|GetActorLocation)))

(event Collision|EventActorBeginOverlap
  (params (OtherActor :type Actor%20Object%20Reference)))

(event EventTick
  (params (DeltaSeconds :type Float%20%28single-precision%29))
  (Transformation|SetActorLocation (+ (+ (Variables|Default|GetOrigin) "") (* (Transformation|GetActorUpVector) (Math|Curves|GetFloatValue (Variables|Default|GetNewVar) (Utilities|Time|GetTimeSeconds)) 1e+02)) false false))

(fn ConstructionScript)