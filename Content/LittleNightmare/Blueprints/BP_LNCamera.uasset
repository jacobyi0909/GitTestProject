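; BP_LNCamera is a follow camera for LittleNightmare that keeps a fixed offset from the player.
; On BeginPlay it becomes the player controller's view target, caches the player pawn and records its starting offset from that pawn.
; Each Tick it moves to the pawn's location plus that offset without sweeping, leaving rotation untouched, so the placement in the level defines the framing.
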(event EventBeginPlay
  (Game|Player|SetViewTargetwithBlend (Game|GetPlayerController 0) self 0.0 "VTBlend_Linear" 0.0 false)
  (bind _output_get (Variables|Default|SetPlayer (Game|Player|GetPlayerPawn 0)))
  (Variables|Default|SetOffset (- (Transformation|GetActorLocation) (Transformation|GetActorLocation _output_get))))

(event Collision|EventActorBeginOverlap
  (params (OtherActor :type Actor%20Object%20Reference)))

(event EventTick
  (params (DeltaSeconds :type Float%20%28single-precision%29))
  (Transformation|SetActorLocation (+ (Transformation|GetActorLocation (Variables|Default|GetPlayer)) (Variables|Default|GetOffset)) false false))

(fn ConstructionScript)