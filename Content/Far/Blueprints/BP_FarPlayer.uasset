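; BP_FarPlayer is a player Blueprint with two custom events that trace from the camera and hide the components they hit.
; FindLineTrace casts a visibility line, prints the hit component's name, hides it and re-shows the previously stored one, only when something is hit.
; FindMultiSphereTrace sweeps a shorter sphere trace, re-showing all previous hits before hiding the new set.
; Both draw debug traces, and nothing here calls them.
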(event Custom|FindMultiSphereTrace
  (bind _camera (Variables|Default|GetCamera))
  (bind _returnvalue (Transformation|GetWorldLocation _camera))
  (bind _outhits (Collision|MultiSphereTraceByChannel _returnvalue (+ _returnvalue (* (Math|Vector|GetForwardVector _camera) 3e+02)) (Variables|Default|GetRadius) "TraceTypeQuery1" false 0 "ForOneFrame"))
  (for _array_element (Variables|Default|GetChooseComponents)
    (Rendering|SetVisibility (.HitComponent (Collision|BreakHitResult _array_element)) true false))
  (bind _output_get (Variables|Default|SetChooseComponents _outhits))
  (for _array_element_2 _output_get
    (Rendering|SetVisibility (.HitComponent (Collision|BreakHitResult _array_element_2)) false false)))

(event Custom|FindLineTrace
  (bind _camera (Variables|Default|GetCamera))
  (bind _returnvalue (Transformation|GetWorldLocation _camera))
  (bind (_outhit _returnvalue_2) (Collision|LineTraceByChannel _returnvalue (+ _returnvalue (* (Math|Vector|GetForwardVector _camera) 1e+03)) "TraceTypeQuery1" false 0 "ForOneFrame"))
  (if _returnvalue_2
    (Development|PrintString (Utilities|GetDisplayName (.HitComponent (Collision|BreakHitResult _outhit))))
    (bind _choosecomponent (Variables|Default|GetChooseComponent)
      (:then
        (Rendering|SetVisibility _choosecomponent true false))
      (:else
        _))
    (bind _output_get (Variables|Default|SetChooseComponent (.HitComponent (Collision|BreakHitResult _outhit))))
    (Rendering|SetVisibility _output_get false false)))

(event EventBeginPlay)

(event Collision|EventActorBeginOverlap
  (params (OtherActor :type Actor%20Object%20Reference)))

(event EventTick
  (params (DeltaSeconds :type Float%20%28single-precision%29)))

(fn ConstructionScript)