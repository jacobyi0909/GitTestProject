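; BP_CrossProductTest is a test Blueprint that visualizes the cross product of two vectors, A and B.
; Every tick it computes A × B by hand, component by component, rather than with the built-in node.
; It then sets the Scene component's world rotation so its X axis points along the resulting vector.
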(event EventBeginPlay)

(event Collision|EventActorBeginOverlap
  (params (OtherActor :type Actor%20Object%20Reference)))

(event EventTick
  (params (DeltaSeconds :type Float%20%28single-precision%29))
  (bind _a (Variables|Default|Geta))
  (bind _b (Variables|Default|Getb))
  (bind _a_2 (Variables|Default|Geta))
  (bind _b_2 (Variables|Default|Getb))
  (bind _output_get (Variables|Default|SetDir (Math|Vector|MakeVector (- (* (.y _a_2) (.z _b_2)) (* (.z _a) (.y _b))) (- (* (.z _a_2) (.x _b_2)) (* (.x _a) (.z _b))) (- (* (.x _a_2) (.y _b_2)) (* (.y _a) (.x _b))))))
  (Transformation|SetWorldRotation (Variables|Default|GetScene) (Math|Rotator|MakeRotfromX (- _output_get "")) false false))

(fn ConstructionScript)